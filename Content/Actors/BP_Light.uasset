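; BP_Light is a light actor whose spotlight switches on and off with the game world's time.
; BeginPlay caches a BP_GameMode reference, and every Tick runs a SetVisibility event that reads its WorldTime.
; The spotlight is visible while WorldTime is between 9 and 15 inclusive and hidden otherwise, although the Tick logic is labeled as a night-time check.
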(event Custom|SetVisibility
  (bind _gamemoderef (Variables|Default|GetGameModeRef))
  (bind _worldtime (Variables|/Game/BP_GameMode.BP_GameMode_C|GetWorldTime _gamemoderef))
  ;[0 1 0.06881 1 30] CheckNightTime
  (if (and (>= _worldtime 9.0) (<= _worldtime 15.0))
    (Rendering|SetVisibility (Variables|Default|GetSpotLight) true false)
    (else
      (Rendering|SetVisibility (Variables|Default|GetSpotLight) false false))))

(event EventTick
  (params (DeltaSeconds :type Float%20%28single-precision%29))
  ;[0 1 0.06881 1 30] CheckNightTime
  (CallFunction|SetVisibility))

(event EventBeginPlay
  (bind _asbp_game_mode (Utilities|Casting|CastToBP_GameMode (Game|GetGameMode)))
  (Variables|Default|SetGameModeRef _asbp_game_mode))

(fn ConstructionScript)