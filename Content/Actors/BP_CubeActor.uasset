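; BP_CubeActor is an actor that moves along a referenced spline and displays its own name on a widget.
; A MoveCube event, with no caller in this graph, advances travelled distance by delta times speed and places the actor at that world-space spline point.
; On passing the spline's end, the distance wraps and that call skips the location update.
; BeginPlay writes the actor's display name into its UW_Icon widget.
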(event Custom|MoveCube
  (params (Delta :type Float%20%28double-precision%29))
  (bind _splineref (Variables|Default|GetSplineRef))
  (bind _returnvalue (Spline|GetSplineLength _splineref))
  ;[0 1 0.03955 1 30] MoveCubeFunc
  (bind _output_get (Variables|Default|SetDistanceTraveled (+ (* Delta (Variables|Default|GetSpeed)) (Variables|Default|GetDistanceTraveled))))
  (if (> _output_get _returnvalue)
    (Variables|Default|SetDistanceTraveled (- (Variables|Default|GetDistanceTraveled) _returnvalue))
    (else
      (Transformation|SetActorLocation (Spline|GetLocationatDistanceAlongSpline (Variables|Default|GetSplineRef) (Variables|Default|GetDistanceTraveled) "World") false false))))

(event EventBeginPlay
  (bind _asuw_icon (Utilities|Casting|CastToUW_Icon (UserInterface|GetUserWidgetObject (Variables|Default|GetWidget))))
  (Variables|/Script/UMG.TextBlock|SetText (Variables|/Game/Actors/Widget/UW_Icon.UW_Icon_C|GetActorNameText _asuw_icon) (Utilities|Text|ToText(String) (Utilities|GetDisplayName self))))

(fn ConstructionScript)